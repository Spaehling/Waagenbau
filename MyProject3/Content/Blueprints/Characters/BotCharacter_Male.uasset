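; Male bot character Blueprint with per-instance clothing, hair and handheld props, whose state variables suggest a bar or party crowd NPC.
; The construction script builds dynamic material instances for shirt, pants and hair from color, texture and normal variables.
; It also sets bottle and cigarette meshes and toggles their visibility, plus that of the hand and mouth smoke components.
; Tick continuously sets max walk speed to SpeedRate times SpeedVariable.
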(event `self.ReceiveTick`
  (params (DeltaSeconds :type "Float (single-precision)"))
  (set `CharacterMovementComponent.MaxWalkSpeed` (* (`self.SpeedRate`) (`self.SpeedVariable`)) (`self.CharacterMovement`)))

(fn `UserConstructionScript`
  (bind _bottle_on_off (`self.Bottle On/Off`))
  (bind _set_pants_color (`self.Set Pants Color`))
  (bind _set_3_hair_color (`self.Set 3 Hair Color`))
  (bind _bottle (`self.Bottle`))
  (bind _cigarette_on_off (`self.Cigarette On/Off`))
  (bind _cigarette (`self.Cigarette`))
  (bind _set_1_hair_color (`self.Set 1 Hair Color`))
  (bind _set_2_hair_color (`self.Set 2 Hair Color`))
  (bind _set_shirt_color (`self.Set Shirt Color`))
  ;[1 1 1] Shirt
  (bind _returnvalue (`KismetMaterialLibrary.CreateDynamicMaterialInstance` "/Game/Materials/Cloth/tshirt_Inst.tshirt_Inst"))
  (set `self.Set Material Instance` _returnvalue)
  (`PrimitiveComponent.SetMaterial` (`self.Mesh`) 0 (`self.Set Material Instance`))
  (set `self.Set Shirt Color` _set_shirt_color)
  (`MaterialInstanceDynamic.SetVectorParameterValue` (`self.Set Material Instance`) "TShirtColor" _set_shirt_color)
  (`MaterialInstanceDynamic.SetTextureParameterValue` (`self.Set Material Instance`) "Texture" (`self.Set Shirt Texture`))
  (`MaterialInstanceDynamic.SetTextureParameterValue` (`self.Set Material Instance`) "TShirtNormal" (`self.Set Shirt Normal`))
  ;[1 1 1] Pants
  (bind _returnvalue_2 (`KismetMaterialLibrary.CreateDynamicMaterialInstance` "/Game/Materials/Cloth/pants_1_Inst.pants_1_Inst"))
  (set `self.Set Material Instance` _returnvalue_2)
  (`PrimitiveComponent.SetMaterial` (`self.Mesh`) 6 (`self.Set Material Instance`))
  (set `self.Set Pants Color` _set_pants_color)
  (`MaterialInstanceDynamic.SetVectorParameterValue` (`self.Set Material Instance`) "TShirtColor" _set_pants_color)
  (`MaterialInstanceDynamic.SetTextureParameterValue` (`self.Set Material Instance`) "Texture" (`self.Set Pants Texture`))
  (`MaterialInstanceDynamic.SetTextureParameterValue` (`self.Set Material Instance`) "TShirtNormal" (`self.Set Pants Normal`))
  ;[1 1 1] Hair
  (bind _returnvalue_3 (`KismetMaterialLibrary.CreateDynamicMaterialInstance` "/Game/Materials/Char/hair_Inst.hair_Inst"))
  (set `self.Set Material Instance` _returnvalue_3)
  (`PrimitiveComponent.SetMaterial` (`self.Mesh`) 2 (`self.Set Material Instance`))
  (set `self.Set 1 Hair Color` _set_1_hair_color)
  (`MaterialInstanceDynamic.SetVectorParameterValue` (`self.Set Material Instance`) "Hair Main Color" _set_1_hair_color)
  (set `self.Set 2 Hair Color` _set_2_hair_color)
  (`MaterialInstanceDynamic.SetVectorParameterValue` (`self.Set Material Instance`) "Hair Second Color" _set_2_hair_color)
  (set `self.Set 3 Hair Color` _set_3_hair_color)
  (`MaterialInstanceDynamic.SetVectorParameterValue` (`self.Set Material Instance`) "Hair Third Color" _set_3_hair_color)
  (`MaterialInstanceDynamic.SetTextureParameterValue` (`self.Set Material Instance`) "Hair Texture" (`self.Set Hair Texture`))
  (`MaterialInstanceDynamic.SetTextureParameterValue` (`self.Set Material Instance`) "Hair Normal" (`self.Set Hair Normal`))
  ;[1 1 1] Left Hand
  (`StaticMeshComponent.SetStaticMesh` _bottle (`self.Set Bottle`))
  (`SceneComponent.SetVisibility` _bottle _bottle_on_off false)
  (set `self.Bottle On/Off` _bottle_on_off)
  (set `self.Drink On/Off` (`self.Drink On/Off`))
  (set `self.Dancing High` (`self.Dancing High`))
  (set `self.Standing at bar` (`self.Standing at bar`))
  ;[1 1 1] Right Hand
  (`StaticMeshComponent.SetStaticMesh` _cigarette (`self.Set Cigarette`))
  (`SceneComponent.SetVisibility` _cigarette _cigarette_on_off false)
  (set `self.Cigarette On/Off` _cigarette_on_off)
  (`SceneComponent.SetVisibility` (`self.Hand`) (`self.Smoke Visible?`) false)
  (`SceneComponent.SetVisibility` (`self.Mouth`) (`self.Smoke Visible?`) false)
  (set `self.Smoke On/Off` (`self.Smoke On/Off`))
  (set `self.Smoke Walk On/Off` (`self.Smoke Walk On/Off`)))