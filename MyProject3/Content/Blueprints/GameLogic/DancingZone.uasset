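; DancingZone is a trigger volume that adjusts dance and drink state flags on male bot characters entering or leaving it.
; Begin overlap prints the bot's name, and both overlap events branch on its dancing flag to clear either that flag or the dance-walking flag.
; Both events also clear the zone's SetDancingInDancingZone flag and sync the bot's bottle flag to its drink flag.
; As written, neither event switches dancing on.
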(event `self.Trigger.OnComponentBeginOverlap`
  (params (OtherActor :type "Actor Object Reference") (OtherComp :type "PrimitiveComponent Object Reference") (OtherBodyIndex :type Integer) (bFromSweep :type Boolean) (SweepResult :type "EngineTypes.HitResult Structure (by ref)"))
  ;[1 1 1] Comment
  (bind _asbotcharacter_male_c (cast `/Game/Blueprints/Characters/BotCharacter_Male` OtherActor))
  (`KismetSystemLibrary.PrintString` (`KismetSystemLibrary.GetDisplayName` _asbotcharacter_male_c))
  (if (`/Game/Blueprints/Characters/BotCharacter_Male.Dancing On/OFf` _asbotcharacter_male_c)
    (set `/Game/Blueprints/Characters/BotCharacter_Male.Dancing Walking on/off` false _asbotcharacter_male_c)
    (else
      (set `/Game/Blueprints/Characters/BotCharacter_Male.Dancing On/OFf` false _asbotcharacter_male_c)))
  (set `self.Set Dancing in DancingZone` false)
  (if (`/Game/Blueprints/Characters/BotCharacter_Male.Drink On/Off` _asbotcharacter_male_c)
    (set `/Game/Blueprints/Characters/BotCharacter_Male.Drink On/Off` true _asbotcharacter_male_c)
    (set `/Game/Blueprints/Characters/BotCharacter_Male.Bottle On/Off` true _asbotcharacter_male_c)
    (else
      (set `/Game/Blueprints/Characters/BotCharacter_Male.Drink On/Off` false _asbotcharacter_male_c)
      (set `/Game/Blueprints/Characters/BotCharacter_Male.Bottle On/Off` false _asbotcharacter_male_c))))

(event `self.Trigger.OnComponentEndOverlap`
  (params (OtherActor :type "Actor Object Reference") (OtherComp :type "PrimitiveComponent Object Reference") (OtherBodyIndex :type Integer))
  ;[1 1 1] Comment
  (bind _asbotcharacter_male_c (cast `/Game/Blueprints/Characters/BotCharacter_Male` OtherActor))
  (if (`/Game/Blueprints/Characters/BotCharacter_Male.Dancing On/OFf` _asbotcharacter_male_c)
    (set `/Game/Blueprints/Characters/BotCharacter_Male.Dancing On/OFf` false _asbotcharacter_male_c)
    (else
      (set `/Game/Blueprints/Characters/BotCharacter_Male.Dancing Walking on/off` false _asbotcharacter_male_c)))
  (set `self.Set Dancing in DancingZone` false)
  (if (`/Game/Blueprints/Characters/BotCharacter_Male.Drink On/Off` _asbotcharacter_male_c)
    (set `/Game/Blueprints/Characters/BotCharacter_Male.Drink On/Off` true _asbotcharacter_male_c)
    (set `/Game/Blueprints/Characters/BotCharacter_Male.Bottle On/Off` true _asbotcharacter_male_c)
    (else
      (set `/Game/Blueprints/Characters/BotCharacter_Male.Drink On/Off` false _asbotcharacter_male_c)
      (set `/Game/Blueprints/Characters/BotCharacter_Male.Bottle On/Off` false _asbotcharacter_male_c))))

(fn `UserConstructionScript`)