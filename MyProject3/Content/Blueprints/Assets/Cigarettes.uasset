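; Cigarette pack prop Blueprint with a configurable color and mesh.
; The Construction Script creates a dynamic material instance from Cigarettes_Mat_Inst, assigns it to the first material slot and feeds the SetPackColor variable into its PackColor parameter.
; It then applies the SetMesh variable to the static mesh component, so one Blueprint covers multiple pack variants.
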(fn `UserConstructionScript`
  (bind _setpackcolor (`self.SetPackColor`))
  ;[1 1 1] Comment
  (bind _returnvalue (`KismetMaterialLibrary.CreateDynamicMaterialInstance` "/Game/Materials/cigarettes_Mat_Inst.cigarettes_Mat_Inst"))
  (set `self.PackColor` _returnvalue)
  (`PrimitiveComponent.SetMaterial` (`self.StaticMesh1`) 0 (`self.PackColor`))
  (set `self.SetPackColor` _setpackcolor)
  (`MaterialInstanceDynamic.SetVectorParameterValue` (`self.PackColor`) "PackColor" _setpackcolor)
  (`StaticMeshComponent.SetStaticMesh` (`self.StaticMesh1`) (`self.Set Mesh`)))