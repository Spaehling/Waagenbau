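; Sound box actor that plays a sound from its Sounds array when play begins.
; BeginPlay plays the entry indexed by NewVar at the world origin, independently of the Audio1 component.
; The construction script assigns Audio1 a sound via RandomInteger(1), which always yields the first entry.
; It then restarts Audio1 if it is already playing, otherwise stops it.
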(event `self.ReceiveBeginPlay`
  (`GameplayStatics.PlaySoundAtLocation` (`KismetArrayLibrary.Array_Get` (`self.Sounds`) (`self.NewVar`))))

(fn `UserConstructionScript`
  (bind _audio1 (`self.Audio1`))
  (`AudioComponent.SetSound` _audio1 (`KismetArrayLibrary.Array_Get` (`self.Sounds`) (`KismetMathLibrary.RandomInteger` 1)))
  (bind _returnvalue (`AudioComponent.IsPlaying` _audio1))
  (if _returnvalue
    (`AudioComponent.Play` _audio1 0.0)
    (else
      (`AudioComponent.Stop` _audio1))))