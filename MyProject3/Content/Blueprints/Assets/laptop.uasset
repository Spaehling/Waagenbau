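; Laptop actor with three text tracks, apparently a selection menu that responds to input near it.
; Its trigger volume enables player input on overlap and disables it on exit.
; Pressing Up tints Track1 blue if Intrigger is true, otherwise whitens all three tracks, as does releasing Up after a one-second delay.
; Intrigger is never set in these graphs, and the Track2 highlight is unconnected.
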(event `self.TriggerVolume.OnComponentBeginOverlap`
  (params (OtherActor :type "Actor Object Reference") (OtherComp :type "PrimitiveComponent Object Reference") (OtherBodyIndex :type Integer))
  (`self.EnableInput` (`GameplayStatics.GetPlayerController` 0)))

(event `self.TriggerVolume.OnComponentEndOverlap`
  (params (OtherActor :type "Actor Object Reference") (OtherComp :type "PrimitiveComponent Object Reference") (OtherBodyIndex :type Integer))
  (`self.DisableInput` (`GameplayStatics.GetPlayerController` 0)))

(event `Key|Up`
  (:`Pressed`
    (if (`self.intrigger`)
      (`TextRenderComponent.SetTextRenderColor` (`self.Track 1`) (`KismetMathLibrary.Conv_LinearColorToColor` (struct :`G` 0.027829 :`B` 1.0 :`A` 1.0)))
      (else
        (`TextRenderComponent.SetTextRenderColor` (`self.Track 1`) (`KismetMathLibrary.Conv_LinearColorToColor` (struct :`R` 1.0 :`G` 1.0 :`B` 1.0 :`A` 1.0)) :!label _label)
        (`TextRenderComponent.SetTextRenderColor` (`self.Track 2`) (`KismetMathLibrary.Conv_LinearColorToColor` (struct :`R` 1.0 :`G` 1.0 :`B` 1.0 :`A` 1.0)))
        (`TextRenderComponent.SetTextRenderColor` (`self.Track 3`) (`KismetMathLibrary.Conv_LinearColorToColor` (struct :`R` 1.0 :`G` 1.0 :`B` 1.0 :`A` 1.0))))))
  (:`Released`
    (`KismetSystemLibrary.Delay` 1.0)
    (goto _label)))

(fn `UserConstructionScript`)