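; DiscoLight_1 is a configurable disco lamp that blinks its spot light, bounce light and light cone mesh at a fixed interval.
; The Construction Script applies color, brightness, cone angles, meshes and default light visibility, and creates dynamic materials for lamp and cone.
; BeginPlay tints both materials with LightColor, then a looping Delay toggles visibility every Time seconds.
; The Construction Script's timer call names no function, so the Delay loop drives the blinking.
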(event `self.ReceiveBeginPlay`
  ;[0.7668 1 0.8796] Plastic Color
  (`MaterialInstanceDynamic.SetVectorParameterValue` (`self.Mat_Inst_Dym_2`) "Plastic Color" (`self.Light Color`))
  ;[0.7668 1 0.8796] Cone Color
  (`MaterialInstanceDynamic.SetVectorParameterValue` (`self.Mat_Inst_Dym`) "Cone Color 1" (`self.Light Color`))
  ;[0.7668 1 0.8796] ON/OFF Time
  (`KismetSystemLibrary.Delay` (`self.Time`) :!label _label)
  (`SceneComponent.ToggleVisibility` (`self.SpotLight`) false)
  (`SceneComponent.ToggleVisibility` (`self.BounceLight`) false)
  (`SceneComponent.ToggleVisibility` (`self.Light Cone`) false)
  (goto _label))

(fn `UserConstructionScript`
  (bind _spotlight (`self.SpotLight`))
  ;[1 1 1] Comment
  (`LightComponent.SetLightColor` _spotlight (`self.Light Color`))
  (`LightComponent.SetLightColor` (`self.BounceLight`) (`self.Light Color`))
  (`SceneComponent.SetVisibility` _spotlight (`self.EnablebyDefault`) false)
  (`SceneComponent.SetVisibility` (`self.BounceLight`) (`self.EnablebyDefault`) false)
  ;[1 1 1] Timer
  (`KismetSystemLibrary.K2_SetTimer` null "" (`self.Time`))
  ;[1 1 1] Plastic Material Color
  (bind _returnvalue (`KismetMaterialLibrary.CreateDynamicMaterialInstance` "/Game/Materials/Instances/Plastic_Foliage_Mat_Inst.Plastic_Foliage_Mat_Inst"))
  (set `self.Mat_Inst_Dym_2` _returnvalue)
  (`PrimitiveComponent.SetMaterial` (`self.Lamp`) 0 (`self.Mat_Inst_Dym_2`))
  ;[1 1 1] Light Cone Color
  (bind _returnvalue_2 (`KismetMaterialLibrary.CreateDynamicMaterialInstance` "/Game/Materials/Instances/light_cone_mat_Inst.light_cone_mat_Inst"))
  (set `self.Mat_Inst_Dym` _returnvalue_2)
  (`PrimitiveComponent.SetMaterial` (`self.Light Cone`) 0 (`self.Mat_Inst_Dym`))
  ;[1 1 1] Inner Cone
  (`SpotLightComponent.SetInnerConeAngle` (`self.SpotLight`) (`self.InnerCone`))
  ;[1 1 1] Outer Cone
  (`SpotLightComponent.SetOuterConeAngle` (`self.SpotLight`) (`self.Outer Cone`))
  ;[1 1 1] Light Intensity
  (`LightComponent.SetBrightness` (`self.SpotLight`) (`self.Light Intensity / Brightness`))
  (`LightComponent.SetBrightness` (`self.BounceLight`) (`self.Light Intensity / Brightness`))
  ;[1 1 1] Set Lamp Mesh
  (`StaticMeshComponent.SetStaticMesh` (`self.Lamp`) (`self.Set Lamp Mesh`))
  ;[1 1 1] Set Cone Mesh
  (`StaticMeshComponent.SetStaticMesh` (`self.Light Cone`) (`self.Set Cone Mesh`)))